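; Dark Tether gameplay ability that slows pawns around a targeted point.
; On activation it gets instant target data from GASTargetActor, centring a sphere overlap on the hit location, or the trace end if nothing blocks.
; Each overlapped pawn with an Ability System Component, excluding the owner, applies GE_DarkTetherSlowSpeed to itself.
; The ability ends after applying the effect or when targeting is cancelled.
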(event Ability|EventActivateAbility
  (bind _data (|WaitTargetData :ConfirmationType "Instant" :Class "/Script/GASReplication.GASTargetActor" :TraceRange 2e+03 :ReticleClass 0)
    (:ValidData
      (bind _outactors (Collision|SphereOverlapActors (Math|Vector|SelectVector (.Location (Collision|BreakHitResult (Ability|TargetData|GetHitResultfromTargetData _data))) (.TraceEnd (Collision|BreakHitResult (Ability|TargetData|GetHitResultfromTargetData _data))) (.bBlockingHit (Collision|BreakHitResult (Ability|TargetData|GetHitResultfromTargetData _data)))) 5e+02 (Utilities|Array|MakeArray "ObjectTypeQuery3") 0 (Utilities|Array|MakeArray (Ability|GetOwningActorfromActorInfo))))
      (for _array_element _outactors
        (Utilities|IsValid (Ability|GetAbilitySystemComponent _array_element)
          (:Is%20Valid
            (GameplayEffects|ApplyGameplayEffectToSelf :self (Ability|GetAbilitySystemComponent _array_element) :GameplayEffectClass "/Game/GAS/Abilities/2_DarkTether/GE_DarkTetherSlowSpeed.GE_DarkTetherSlowSpeed_C")
            (Development|PrintString "Effect Applied"))))
      (Ability|EndAbility))
    (:Cancelled
      (Ability|EndAbility))))