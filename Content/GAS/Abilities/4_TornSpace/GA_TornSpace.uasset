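; Torn Space gameplay ability that quickly moves the owning actor to a player-targeted point.
; WaitTargetData spawns GASTargetActor with the GARet_TornSpace reticle and flags the owner as targeting until the ability ends.
; On confirmation, a short MoveToLocation task heads to the hit location, or to the trace end when nothing blocks.
; On arrival it fires the tornSpace gameplay cue at the owner's location and ends; cancelling ends it immediately.
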(event Ability|EventActivateAbility
  (bind _data (|WaitTargetData :ConfirmationType "UserConfirmed" :Class "/Script/GASReplication.GASTargetActor" :ReticleClass "/Game/GAS/Abilities/4_TornSpace/GARet_TornSpace.GARet_TornSpace_C")
    (:then
      (Class|BPIAbilityInterface|SetIsTargeting(Message) (Ability|GetOwningActorfromActorInfo) true))
    (:ValidData
      (AI|Navigation|MovetoLocation "None" (Math|Vector|SelectVector (.Location (Collision|BreakHitResult (Ability|TargetData|GetHitResultfromTargetData _data))) (.TraceEnd (Collision|BreakHitResult (Ability|TargetData|GetHitResultfromTargetData _data))) (.bBlockingHit (Collision|BreakHitResult (Ability|TargetData|GetHitResultfromTargetData _data)))) 0.2
        (:OnTargetLocationReached
          (Class|GameplayAbility|ExecuteGameplayCuewithParams "(TagName=\"GameplayCue.ability.tornSpace.cueEffect\")" (Ability|GameplayCue|MakeGameplayCueParameters :Location (Transformation|GetActorLocation (Ability|GetOwningActorfromActorInfo))))
          (Ability|EndAbility))))
    (:Cancelled
      (Ability|EndAbility))))

(event Ability|EventOnEndAbility
  (params (bWasCancelled :type Boolean))
  (Class|BPIAbilityInterface|SetIsTargeting(Message) (Ability|GetOwningActorfromActorInfo) false))