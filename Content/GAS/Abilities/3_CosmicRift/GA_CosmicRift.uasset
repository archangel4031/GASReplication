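; GA_CosmicRift is a targeted gameplay ability that calls down a Cosmic Rift meteor at a player-confirmed spot.
; It waits on a GAS target actor with a custom reticle and flags the owner as targeting until the ability ends.
; A blocking hit spawns BP_CosmicRiftMeteor there, handing it an outgoing damage effect spec.
; Invalid hits only print a message, and both confirm and cancel end the ability.
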(event Ability|EventActivateAbility
  (bind _data (|WaitTargetData :ConfirmationType "UserConfirmed" :Class "/Script/GASReplication.GASTargetActor" :TraceRange 2.5e+03 :ReticleClass "/Game/GAS/Abilities/3_CosmicRift/GARet_CosmicRift.GARet_CosmicRift_C")
    (:then
      (Class|BPIAbilityInterface|SetIsTargeting(Message) (Ability|GetOwningActorfromActorInfo) true)
      (Development|PrintString "Targeting Active"))
    (:ValidData
      (if (.bBlockingHit (Collision|BreakHitResult (Ability|TargetData|GetHitResultfromTargetData _data)))
        (Game|SpawnActorfromClass "/Game/GAS/Abilities/3_CosmicRift/BP_CosmicRiftMeteor.BP_CosmicRiftMeteor_C" (Math|Transform|MakeTransform (.Location (Collision|BreakHitResult (Ability|TargetData|GetHitResultfromTargetData _data)))) "AlwaysSpawn" 0 5e+02 (Ability|MakeOutgoingGameplayEffectSpec "/Game/GAS/Abilities/3_CosmicRift/GE_CosmicRiftDamage.GE_CosmicRiftDamage_C") (Variables|/Script/Engine.Actor|GetInstigator (Ability|GetOwningActorfromActorInfo)))
        (else
          (Development|PrintString "Invalid Target")))
      (Ability|EndAbility))
    (:Cancelled
      (Ability|EndAbility))))

(event Ability|EventOnEndAbility
  (params (bWasCancelled :type Boolean))
  (Class|BPIAbilityInterface|SetIsTargeting(Message) (Ability|GetOwningActorfromActorInfo) false))