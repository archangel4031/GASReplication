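; Meteor actor for the Cosmic Rift ability that applies a gameplay effect to pawns around it when it spawns.
; On BeginPlay it runs a sphere overlap of ScanRadius at its location, ignoring its instigator.
; The instigator's Ability System Component applies the stored effect spec to each overlapped pawn that has its own Ability System Component.
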(event EventBeginPlay
  (bind _returnvalue (Game|GetInstigator))
  (bind _outactors (Collision|SphereOverlapActors (Transformation|GetActorLocation) (Variables|Default|GetScanRadius) (Utilities|Array|MakeArray "ObjectTypeQuery3") 0 (Utilities|Array|MakeArray _returnvalue)))
  (for _array_element _outactors
    (Utilities|IsValid (Ability|GetAbilitySystemComponent _array_element)
      (:Is%20Valid
        (GameplayEffects|ApplyGameplayEffectSpecToTarget (Ability|GetAbilitySystemComponent _returnvalue) (Variables|Default|GetEffectSpecHandle) (Ability|GetAbilitySystemComponent _array_element))))))

(fn ConstructionScript)