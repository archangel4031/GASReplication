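; BP_Ultimate is the area-of-effect actor for a GAS ultimate ability, affecting actors inside its Sphere.
; On begin overlap, the instigator's Ability System Component applies EffectSpecHandle to any other actor with an Ability System Component, excluding the instigator.
; On end overlap, it removes effects tagged Char.ability.ultimate.damageEffect from the leaving actor, with no instigator check.
; The spec handle is not built or assigned in these graphs.
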(event OnComponentBeginOverlap(Sphere)
  (params (OverlappedComponent :type Primitive%20Component%20Object%20Reference) (OtherActor :type Actor%20Object%20Reference) (OtherComp :type Primitive%20Component%20Object%20Reference) (OtherBodyIndex :type Integer) (bFromSweep :type Boolean) (SweepResult :type Hit%20Result%20Structure%20%28by%20ref%29))
  (bind _returnvalue (Game|GetInstigator))
  (bind _returnvalue_2 (Ability|GetAbilitySystemComponent OtherActor))
  (if (!= OtherActor _returnvalue)
    (Utilities|IsValid _returnvalue_2
      (:Is%20Valid
        (GameplayEffects|ApplyGameplayEffectSpecToTarget (Ability|GetAbilitySystemComponent _returnvalue) (Variables|Default|GetEffectSpecHandle) _returnvalue_2)))))

(event OnComponentEndOverlap(Sphere)
  (params (OverlappedComponent :type Primitive%20Component%20Object%20Reference) (OtherActor :type Actor%20Object%20Reference) (OtherComp :type Primitive%20Component%20Object%20Reference) (OtherBodyIndex :type Integer))
  (bind _returnvalue (Ability|GetAbilitySystemComponent OtherActor))
  (Utilities|IsValid _returnvalue
    (:Is%20Valid
      (GameplayEffects|RemoveActiveEffectswithTags _returnvalue "(GameplayTags=((TagName=\"char.ability.ultimate.damageEffect\")))"))))

(fn ConstructionScript)